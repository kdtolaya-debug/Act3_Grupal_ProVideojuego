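; Enemy character that chases and melee-attacks the first player's character once Pawn Sensing spots a pawn.
; Each sighting sets EstaViendoAlJugador and calls FollowPlayer, which re-arms PuedeAtacar and runs AIMoveTo toward the player.
; On arrival it plays an attack montage, applies damage immediately and delays re-arming by the montage length.
; Tick halts movement until the first sighting; the seen flag is never effectively cleared afterward.
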(event OnSeePawn(PawnSensing)
  (params (Pawn :type Pawn%20Object%20Reference))
  (Variables|Default|SetEstaViendoAlJugador? true)
  (CallFunction|FollowPlayer))

(event Custom|FollowPlayer
  (Variables|Default|SetPuedeAtacar true)
  (if (Variables|Default|GetEstaViendoAlJugador?)
    (AI|AIMoveTo self "0, 0, 0" (Game|GetPlayerCharacter 0) 5e+01 false
      (:OnSuccess
        (if (Variables|Default|GetPuedeAtacar)
          (Variables|Default|SetPuedeAtacar false)
          (bind _returnvalue (Animation|PlayAnimMontage "/Game/Characters/Mannequins/Anims/Unarmed/Attack/MM_Attack_01_Montage.MM_Attack_01_Montage" 1.0 "None"))
          (Animation|PlayAnimMontage 0 1.0 "None")
          (Game|Damage|ApplyDamage (Game|GetPlayerCharacter 0) 5e+01 0 0)
          (Utilities|FlowControl|Delay _returnvalue)
          (Variables|Default|SetPuedeAtacar true))))
    (else
      (Variables|Default|SetEstaViendoAlJugador? false))))

(event EventBeginPlay)

(event Collision|EventActorBeginOverlap
  (params (OtherActor :type Actor%20Object%20Reference)))

(event EventTick
  (params (DeltaSeconds :type Float%20%28single-precision%29))
  (if (not (Variables|Default|GetEstaViendoAlJugador?))
    (Components|Movement|StopMovementImmediately (Variables|Character|GetCharacterMovement))))

(fn ConstructionScript)